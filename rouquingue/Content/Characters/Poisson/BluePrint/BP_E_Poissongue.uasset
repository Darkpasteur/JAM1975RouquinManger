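; BP_E_Poissongue is a fish actor that patrols side to side along Y between two randomized points, flipping its rotation at each end.
; Tick teleports it each frame unless the player's PAUSEEE flag is set, snapping it to the player when Graillable is false.
; While StunTime counts down, patrol stops, and a Projectile fish flies toward Destination at a speed scaled by the player's JawSpeedLevel.
; Overlap only prints a debug string.
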(event `self.ReceiveBeginPlay`
  (bind (_returnvalue_x _returnvalue_y _returnvalue_z) (`KismetMathLibrary.BreakVector` (`self.K2_GetActorLocation`)))
  (`parent.ReceiveBeginPlay`)
  (set `self.Point gauche` (`KismetMathLibrary.MakeVector` 1000.0 (- _returnvalue_y (`KismetMathLibrary.RandomFloatInRange` 200.0 700.0)) _returnvalue_z))
  (set `self.Point Droit` (`KismetMathLibrary.MakeVector` 1000.0 (+ _returnvalue_y (`KismetMathLibrary.RandomFloatInRange` 200.0 700.0)) _returnvalue_z))
  (bind _output_get (set `self.MoveLeft` (`KismetMathLibrary.RandomBool`)))
  (if _output_get
    (`self.K2_SetActorRotation` (struct) true)
    (else
      (`self.K2_SetActorRotation` (struct :`Yaw` -180.0) true))))

(event `self.ReceiveActorBeginOverlap`
  (params (OtherActor :type "Actor Object Reference"))
  (`parent.ReceiveActorBeginOverlap` OtherActor)
  (`KismetSystemLibrary.PrintString` "poissonqué"))

(event `self.ReceiveTick`
  (params (DeltaSeconds :type "Float (single-precision)"))
  (bind (_returnvalue_x _returnvalue_y) (`KismetMathLibrary.BreakVector` (`self.K2_GetActorLocation`)))
  (bind (_returnvalue_x_2 _returnvalue_y_2 _returnvalue_z) (`KismetMathLibrary.BreakVector` (`self.K2_GetActorLocation`)))
  (bind (_returnvalue_x_3 _returnvalue_y_3) (`KismetMathLibrary.BreakVector` (`self.K2_GetActorLocation`)))
  (bind _returnvalue (`self.K2_GetActorLocation`))
  (bind (_returnvalue_x_4 _returnvalue_y_4 _returnvalue_z_2) (`KismetMathLibrary.BreakVector` (`self.K2_GetActorLocation`)))
  (bind (_point_gauche_x _point_gauche_y) (`KismetMathLibrary.BreakVector` (`self.Point gauche`)))
  (bind (_point_droit_x _point_droit_y) (`KismetMathLibrary.BreakVector` (`self.Point Droit`)))
  (`parent.ReceiveTick` DeltaSeconds)
  (if (<= (`self.StunTime`) 0.0)
    (bind _asbp_top_down_character (cast `/Game/TopDown/Blueprints/BP_TopDownCharacter` (`GameplayStatics.GetPlayerCharacter` 0)))
    (if (`/Game/TopDown/Blueprints/BP_TopDownCharacter.PAUSEEE` _asbp_top_down_character)
      _
      (elif (`self.Graillable`)
        (if (`self.MoveLeft`)
          (if (< _returnvalue_y_3 _point_gauche_y)
            (set `self.MoveLeft` false)
            (`self.K2_SetActorRotation` (struct :`Yaw` -180.0) true)
            (else
              (`self.K2_TeleportTo` (`KismetMathLibrary.MakeVector` 1000.0 (+ _returnvalue_y_2 (* (`self.Speed`) -1.0)) _returnvalue_z) (`self.K2_GetActorRotation`))))
          (elif (> _returnvalue_y _point_droit_y)
            (set `self.MoveLeft` true)
            (`self.K2_SetActorRotation` (struct) true)
            (else
              (`self.K2_TeleportTo` (`KismetMathLibrary.MakeVector` 1000.0 (+ _returnvalue_y_4 (* (`self.Speed`) 1.0)) _returnvalue_z_2) (`self.K2_GetActorRotation`)))))
        (else
          (`self.K2_TeleportTo` (`self.K2_GetActorLocation` (`GameplayStatics.GetPlayerCharacter` 0))))))
    (else
      (set `self.StunTime` (+ (`self.StunTime`) -1.0))
      (if (`self.Projectile`)
        (bind _asbp_top_down_character_2 (cast `/Game/TopDown/Blueprints/BP_TopDownCharacter` (`GameplayStatics.GetPlayerCharacter` 0)))
        (bind _returnvalue_2 (* (+ (/ (`/Game/TopDown/Blueprints/BP_TopDownCharacter.JawSpeedLevel` _asbp_top_down_character_2) 3) 1) 15))
        (`self.K2_TeleportTo` (+ (* (`KismetMathLibrary.Normal` (- (`self.Destination`) _returnvalue)) (`KismetMathLibrary.MakeVector` _returnvalue_2 _returnvalue_2 _returnvalue_2)) _returnvalue))))))

(fn `UserConstructionScript`
  (`parent.UserConstructionScript`))